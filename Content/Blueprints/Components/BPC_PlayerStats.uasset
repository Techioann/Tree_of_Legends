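; Player stats component that tracks health, stamina and money through add and subtract functions.
; Health and money changes push to the WHUD widget, while stamina has no HUD update here.
; Health gains and stamina changes apply one fixed-step FInterpTo per call, so they move only partway toward the target unless clamped.
; Health caps at a hardcoded 100, and its decrease bar divides by MaxStamina instead of MaxHealth.
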(fn `Health Decrease`
  (params (`Damage Health` :type "Float (double-precision)"))
  (bind _output_get (set `self.Health` (- (`self.Health`) `Damage Health`)))
  (if (<= _output_get 0.0)
    (set `self.Health` 0.0))
  (`ProgressBar.SetPercent` (`/Game/UI/WBP_HUD.Health` (`self.W_HUD`)) (/ (`self.Health`) (`self.Max Stamina`))))

(fn `Health Increase`
  (params (`Add Health` :type "Float (double-precision)"))
  (bind _output_get (set `self.ValueHealth` (+ (`self.Health`) `Add Health`)))
  (if (>= _output_get (`self.Max Health`))
    (set `self.Health` 100.0)
    (else
      (set `self.Health` (`KismetMathLibrary.FInterpTo` (`self.Health`) _output_get 0.01 10.0))))
  (`ProgressBar.SetPercent` (`/Game/UI/WBP_HUD.Health` (`self.W_HUD`)) (/ (`self.Health`) (`self.Max Health`))))

(fn `Money Add`
  (params (`Money ADD` :type "Float (double-precision)"))
  (bind _output_get (set `self.Money Current` (+ (`self.Money Current`) `Money ADD`)))
  (`TextBlock.SetText` (`/Game/UI/WBP_HUD.T_Coins` (`self.W_HUD`)) (`KismetTextLibrary.Conv_DoubleToText` _output_get "HalfToEven")))

(fn `Money Sub`
  (params (`Money SUB` :type "Float (double-precision)"))
  (bind _output_get (set `self.Money Current` (- (`self.Money Current`) `Money SUB`)))
  (if (<= _output_get 0.0)
    (set `self.Money Current` 0.0))
  (`TextBlock.SetText` (`/Game/UI/WBP_HUD.T_Coins` (`self.W_HUD`)) (`KismetTextLibrary.Conv_DoubleToText` _output_get "HalfToEven")))

(fn `Stamina Decrease`
  (params (`Decrease Stamina` :type "Float (double-precision)"))
  (bind _output_get (set `self.ValueStamina` (- (`self.Stamina`) `Decrease Stamina`)))
  (if (<= _output_get 0.0)
    (set `self.Stamina` 0.0)
    (else
      (set `self.Stamina` (`KismetMathLibrary.FInterpTo` (`self.Stamina`) (`self.ValueStamina`) 0.01 10.0)))))

(fn `Stamina Increase`
  (params (`Add Stamina` :type "Float (double-precision)"))
  (bind _returnvalue (+ `Add Stamina` (`self.Stamina`)))
  (set `self.ValueStamina` _returnvalue)
  (if (>= _returnvalue (`self.Max Stamina`))
    (set `self.Stamina` (`self.Max Stamina`))
    (else
      (set `self.Stamina` (`KismetMathLibrary.FInterpTo` (`self.Stamina`) (`self.ValueStamina`) 0.01 10.0)))))