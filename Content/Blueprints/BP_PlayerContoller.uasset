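; Player controller that registers the Enhanced Input mapping context on BeginPlay and toggles the menu widget.
; IA_Menu flips IsActiveMenu, either creating a fresh WB_Menus on screen or removing the stored one.
; Opening shows and centers the cursor and switches to UI-only input focused on the menu; the closing branch hides it and restores game-only input.
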(event `self.ReceiveBeginPlay`
  (bind _returnvalue (subsystem `EnhancedInputLocalPlayerSubsystem`))
  ; Add mapping
  (`/Engine/EditorBlueprintResources/StandardMacros.IsValid` _returnvalue
    (:`Is Valid`
      (`EnhancedInputSubsystemInterface.AddMappingContext` _returnvalue "/Game/Inputs/IMC_Mapping.IMC_Mapping" 0 (struct)))))

(event `EnhancedInput|/Game/Inputs/Keys/IA_Menu`
  (params (ActionValue :type Boolean) (ElapsedSeconds :type "Float (double-precision)") (TriggeredSeconds :type "Float (double-precision)") (InputAction :type "InputAction Object Reference" :default "/Game/Inputs/Keys/IA_Menu.IA_Menu"))
  (bind _returnvalue (`GameplayStatics.GetPlayerController` 0))
  (bind (_sizex _sizey) (`self.GetViewportSize` _returnvalue))
  ; Switch widget
  (:`Started`
    (if (`self.IsActiveMenu?`)
      (set `self.IsActiveMenu?` false)
      (`Widget.RemoveFromParent` (`self.W_Menu`))
      (set `PlayerController.bShowMouseCursor` false _returnvalue)
      (`WidgetBlueprintLibrary.SetInputMode_GameOnly` _returnvalue)
      (else
        (set `self.IsActiveMenu?` true)
        (bind _returnvalue_2 (`|CreateWidget` "/Game/UI/WB_Menus.WB_Menus_C" _returnvalue))
        (bind _output_get (set `self.W_Menu` _returnvalue_2))
        (`UserWidget.AddToViewport` _output_get 0)
        (set `PlayerController.bShowMouseCursor` true _returnvalue)
        (`self.SetMouseLocation` _returnvalue (/ _sizex 2) (/ _sizey 2))
        (`WidgetBlueprintLibrary.SetInputMode_UIOnlyEx` _returnvalue _returnvalue_2 "DoNotLock" true)))))

(fn `UserConstructionScript`)