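; Base Game Instance Blueprint that handles creating multiplayer sessions and joining them through accepted invites.
; CreateSession makes an advanced session with private connection slots, then opens the referenced level as a listen server.
; Accepted session invites trigger a join to the invited session.
; On success, both paths hide the mouse cursor and switch the first player controller to game-only input, with no failure handling.
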(event `Create Session`
  (bind _returnvalue (`GameplayStatics.GetPlayerController` 0))
  (`CreateSessionCallbackProxyAdvanced.CreateAdvancedSession` :`PlayerController` (`GameplayStatics.GetPlayerController` 0) :`PrivateConnections` 100
    (:`OnSuccess`
      (`GameplayStatics.OpenLevelBySoftObjectPtr` "/Game/Maps/World.World" true "?listen")
      (`KismetSystemLibrary.PrintText` "Created session")
      (set `PlayerController.bShowMouseCursor` false _returnvalue)
      (`WidgetBlueprintLibrary.SetInputMode_GameOnly` _returnvalue))))

(event `self.OnSessionInviteAccepted`
  (params (LocalPlayerNum :type Integer) (PersonInvited :type "BPUniqueNetId Structure") (SessionToJoin :type "BlueprintSessionResult Structure (by ref)"))
  (bind _returnvalue (`GameplayStatics.GetPlayerController` 0))
  (`JoinSessionCallbackProxy.JoinSession` (`GameplayStatics.GetPlayerController` 0) SessionToJoin
    (:`OnSuccess`
      (set `PlayerController.bShowMouseCursor` false _returnvalue)
      (`WidgetBlueprintLibrary.SetInputMode_GameOnly` _returnvalue))))