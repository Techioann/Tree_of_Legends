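; Tree actor that swaps its static mesh for a procedural mesh copy at BeginPlay, set up through a CutMeshData object.
; CutMeshData initializes with SourceTree and ProceduralTree; on success the static mesh is copied into the procedural component with collision.
; The source is then hidden with collision disabled, leaving the procedural copy to handle queries and physics.
; If initialization fails, the returned error is printed and no swap occurs.
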(event `self.ReceiveBeginPlay`
  (bind (_outerror _returnvalue) (`TOLCutMeshData.InitializeTree` (`self.CutMeshData`) (`self.SourceTree`) (`self.ProceduralTree`)))
  (if _returnvalue
    (`KismetProceduralMeshLibrary.CopyProceduralMeshFromStaticMeshComponent` (`self.SourceTree`) 0 (`self.ProceduralTree`) true)
    (`SceneComponent.SetVisibility` (`self.SourceTree`) false false)
    (`PrimitiveComponent.SetCollisionEnabled` (`self.SourceTree`) "NoCollision")
    (`PrimitiveComponent.SetCollisionEnabled` (`self.ProceduralTree`) "QueryAndPhysics")
    (else
      (`KismetSystemLibrary.PrintString` _outerror false))))

(fn `UserConstructionScript`)